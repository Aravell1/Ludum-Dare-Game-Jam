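; Player-driven bike and cart for the paperboy game that throws newspapers out to either side.
; An Acceleration timeline supplies throttle for swept forward or reverse movement and scales steering.
; Camera arm yaw sets a looking state that drives the zoom timeline and picks the left or right shooting point.
; Shots aim at a camera trace and consume game-mode ammo, with a debug-drawn path prediction for the left side only.
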(event `InputAxis|MoveForward`
  (params (AxisValue :type "Float (single-precision)"))
  (bind _movement_state (`self.Movement State`))
  (bind _movement_state_2 (`self.Movement State`))
  (bind _movement_direction (`self.Movement Direction`))
  (bind _movement_direction_2 (`self.Movement Direction`))
  (set `self.Forward Axis` AxisValue)
  (if (and (> (`self.Forward Axis`) 0.0) (or (`|EnumEquality` _movement_state_2 "NewEnumerator0") (`|EnumEquality` _movement_state_2 "NewEnumerator1") (`|EnumEquality` _movement_state_2 "NewEnumerator2")) (or (== _movement_direction 0.0) (== _movement_direction 1.0)))
    (set `self.Movement State` "NewEnumerator2")
    (set `self.Movement Direction` 1.0)
    (bind (_direction _throttle) (`Timeline|Acceleration` :!label _label)
      (:`Update`
        (set `self.Throttle` _throttle)
        (set `self.Is Moving` (`|EnumInequality` (`self.Movement State`) "NewEnumerator0"))
        (`SceneComponent.K2_AddLocalOffset` (`self.Bike`) (`KismetMathLibrary.MakeVector` (* (`self.Throttle`) 5.0 (`self.Movement Direction`))) true false))
      (:`Finished`
        (if (== (`KismetMathLibrary.Round` (`KismetMathLibrary.VSize` (`SceneComponent.GetComponentVelocity` (`self.Cart`)))) 0)
          (set `self.Movement State` "NewEnumerator0")
          (set `self.Movement Direction` 0.0)
          (elif (> (`self.Movement Direction`) 0.0)
            (set `self.Movement State` "NewEnumerator2")
            (else
              (set `self.Movement State` "NewEnumerator3"))))))
    (else
      (if (and (< (`self.Forward Axis`) 0.0) (or (`|EnumEquality` _movement_state "NewEnumerator0") (`|EnumEquality` _movement_state "NewEnumerator1") (`|EnumEquality` _movement_state "NewEnumerator3")) (or (== _movement_direction_2 0.0) (== _movement_direction_2 -1.0)))
        (set `self.Movement State` "NewEnumerator3")
        (set `self.Movement Direction` -1.0)
        (if (!= (`self.Forward Axis`) 0.0)
          (goto _label)
          (else
            _)))
      (set `self.Movement State` "NewEnumerator1")
      (if (== (`KismetMathLibrary.Round` (`KismetMathLibrary.VSize` (`SceneComponent.GetComponentVelocity` (`self.Cart`)))) 0)
        (set `self.Movement State` "NewEnumerator0")
        (set `self.Movement Direction` 0.0)
        (`|ExecutionSequence`
          (:`then_0`
            (goto _label :!via `Stop`))
          (:`then_1`
            (goto _label :!via `SetNewTime`)))
        (else
          (goto _label :!via `Reverse`))))))

(event `InputAxis|SteerRight`
  (params (AxisValue :type "Float (single-precision)"))
  (bind _is_moving (`self.Is Moving`))
  (bind _returnvalue (* (`self.Throttle`) AxisValue))
  (`PhysicsConstraintComponent.SetOrientationDriveSLERP` (`self.Hitch`) _is_moving)
  (if _is_moving
    (set `self.Turning Rate` _returnvalue)
    (`SceneComponent.K2_AddLocalRotation` (`self.Bike`) (`KismetMathLibrary.MakeRotator` 0.0 0.0 _returnvalue) false false)))

(event `InputAxis|Look Up / Mouse`
  (params (AxisValue :type "Float (single-precision)"))
  (bind _camera (`self.Camera`))
  (bind (_relativerotation_roll _relativerotation_pitch) (`KismetMathLibrary.BreakRotator` (`SceneComponent.RelativeRotation` _camera)))
  (`SceneComponent.K2_SetRelativeRotation` _camera (`KismetMathLibrary.MakeRotator` 0.0 (`KismetMathLibrary.FClamp` (+ _relativerotation_pitch (* AxisValue 5.0)) -10.0 20.0)) false false))

(event `InputAxis|Turn / Mouse`
  (params (AxisValue :type "Float (single-precision)"))
  (`SceneComponent.K2_AddLocalRotation` (`self.Camera Arm`) (`KismetMathLibrary.MakeRotator` 0.0 0.0 (* AxisValue 5.0)) false false))

(event `self.ReceiveTick`
  (params (DeltaSeconds :type "Float (single-precision)"))
  (bind _camera_arm (`self.Camera Arm`))
  (`self.Determine Where Looking`)
  (`self.Predict Paper Shot`)
  (switch `/Game/PaperBoys/CartLooking` (`self.Cart Looking State`)
    (:`NewEnumerator0`
      (`|ExecutionSequence`
        (:`then_0`
          (bind (_direction _camera_arm_length _camera_offset_vector) (`Timeline|CameraZoom` :!via `Stop` :!label _label_2)
            (:`Update`
              (set `SpringArmComponent.TargetArmLength` _camera_arm_length _camera_arm)
              (`SceneComponent.K2_SetRelativeLocation` _camera_arm _camera_offset_vector false false))))
        (:`then_1`
          (goto _label_2))))
    (:`NewEnumerator1`
      (`|ExecutionSequence` :!label _label_3
        (:`then_0`
          (goto _label_2 :!via `Stop`))
        (:`then_1`
          (goto _label_2 :!via `Reverse`))))
    (:`NewEnumerator2`
      (goto _label_3))))

(event `InputAction|Shoot`
  (params (Key :type "Key Structure"))
  (bind _camera (`self.Camera`))
  (bind _papergun_audio_component (`self.PaperGun Audio Component`))
  (bind _camera_2 (`self.Camera`))
  (bind _returnvalue (`SceneComponent.K2_GetComponentLocation` (`self.Right Shooting Point`)))
  (bind _returnvalue_2 (`SceneComponent.K2_GetComponentLocation` (`self.Left Shooting Point`)))
  (bind _returnvalue_3 (`SceneComponent.K2_GetComponentLocation` _camera_2))
  (:`Pressed`
    (if (> (`/Game/PaperBoys/GM_PaperBoy.Newspaper Ammo` (cast `/Game/PaperBoys/GM_PaperBoy` (`GameplayStatics.GetGameMode`) :!pure true)) 0)
      (if (and (`|EnumInequality` (`self.Cart Looking State`) "NewEnumerator0") (`self.Can Fire`))
        (set `self.Can Fire` false)
        (bind (_outhit _returnvalue_4) (`KismetSystemLibrary.LineTraceSingle` _returnvalue_3 (+ _returnvalue_3 (* (`SceneComponent.GetForwardVector` _camera_2) 2500.0)) "TraceTypeQuery1"))
        (if _returnvalue_4
          (set `self.Shooting Location` (`.Location` (`GameplayStatics.BreakHitResult` _outhit)))
          (else
            (set `self.Shooting Location` (+ (`SceneComponent.K2_GetComponentLocation` _camera) (* (`SceneComponent.GetForwardVector` _camera) 2500.0)))))
        (switch `/Game/PaperBoys/CartLooking` (`self.Cart Looking State`)
          (:`NewEnumerator1`
            (`|SpawnActorFromClass` "/Game/PaperBoys/BP_Newspaper.BP_Newspaper_C" (`KismetMathLibrary.MakeTransform` _returnvalue_2 (`KismetMathLibrary.Conv_VectorToRotator` (- (`self.Shooting Location`) _returnvalue_2)) (1.5 1.5 1.5)) "Undefined" "OverrideRootScale" null self))
          (:`NewEnumerator2`
            (`|SpawnActorFromClass` "/Game/PaperBoys/BP_Newspaper.BP_Newspaper_C" (`KismetMathLibrary.MakeTransform` _returnvalue (`KismetMathLibrary.Conv_VectorToRotator` (- (`self.Shooting Location`) _returnvalue)) (1.5 1.5 1.5)) "Undefined" "OverrideRootScale" null self)))
        (`GameplayStatics.SpawnSoundAttached` "/Game/PaperBoys/Sounds/SC_PaperGun.SC_PaperGun" _papergun_audio_component "None" (`SceneComponent.K2_GetComponentLocation` _papergun_audio_component) (struct) "KeepRelativeOffset" false 1.0 1.0 0.0 null null)
        (`/Engine/EditorBlueprintResources/StandardMacros.DecrementInt` (`/Game/PaperBoys/GM_PaperBoy.Newspaper Ammo` (cast `/Game/PaperBoys/GM_PaperBoy` (`GameplayStatics.GetGameMode`) :!pure true))
          (:`  `
            (`KismetSystemLibrary.Delay` 0.01)
            (set `self.Can Fire` true)))))))

(fn `Determine Where Looking`
  (bind (_relativerotation_roll _relativerotation_pitch _relativerotation_yaw) (`KismetMathLibrary.BreakRotator` (`SceneComponent.RelativeRotation` (`self.Camera Arm`))))
  (bind (_relativerotation_roll_2 _relativerotation_pitch_2 _relativerotation_yaw_2) (`KismetMathLibrary.BreakRotator` (`SceneComponent.RelativeRotation` (`self.Camera Arm`))))
  (bind (_relativerotation_roll_3 _relativerotation_pitch_3 _relativerotation_yaw_3) (`KismetMathLibrary.BreakRotator` (`SceneComponent.RelativeRotation` (`self.Camera Arm`))))
  (if (and (>= _relativerotation_yaw -20.0) (<= _relativerotation_yaw 20.0))
    (set `self.Cart Looking State` "NewEnumerator0")
    (elif (and (>= _relativerotation_yaw_2 -179.0) (<= _relativerotation_yaw_2 -21.0))
      (set `self.Cart Looking State` "NewEnumerator1")
      (elif (and (>= _relativerotation_yaw_3 21.0) (<= _relativerotation_yaw_3 179.0))
        (set `self.Cart Looking State` "NewEnumerator2")))))

(fn `Predict Paper Shot`
  (bind _camera (`self.Camera`))
  (bind _camera_2 (`self.Camera`))
  (bind _returnvalue (`SceneComponent.K2_GetComponentLocation` (`self.Left Shooting Point`)))
  (bind _returnvalue_2 (`SceneComponent.K2_GetComponentLocation` _camera_2))
  (bind (_outhit _returnvalue_3) (`KismetSystemLibrary.LineTraceSingle` _returnvalue_2 (+ _returnvalue_2 (* (`SceneComponent.GetForwardVector` _camera_2) 2500.0)) "TraceTypeQuery1"))
  (if _returnvalue_3
    (set `self.Shooting Location` (`.Location` (`GameplayStatics.BreakHitResult` _outhit)))
    (else
      (set `self.Shooting Location` (+ (`SceneComponent.K2_GetComponentLocation` _camera) (* (`SceneComponent.GetForwardVector` _camera) 2500.0)))))
  (switch `/Game/PaperBoys/CartLooking` (`self.Cart Looking State`)
    (:`NewEnumerator1`
      (`GameplayStatics.Blueprint_PredictProjectilePath_ByTraceChannel` _returnvalue (* (- (`self.Shooting Location`) _returnvalue) 4000.0) true 10.0 "ECC_WorldDynamic" true (`|MakeArray` self) "ForOneFrame" 0.0 60.0 1.0 3.0))))

(fn `UserConstructionScript`)