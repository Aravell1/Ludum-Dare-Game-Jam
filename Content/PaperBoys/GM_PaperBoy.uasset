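; GM_PaperBoy is the game mode for a paperboy game, tracking score, remaining time and newspaper ammo to decide when the game ends.
; AddScore accumulates points, while Tick counts down the timer and ends the game at zero, or after a short delay once ammo runs out.
; CompletedGame flags completion, pauses the game, clears all widgets and shows the WBP_Gameover screen.
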(event `Add Score`
  (params (`Delta Score` :type Integer))
  (set `self.Score` (+ (`self.Score`) `Delta Score`)))

(event `self.ReceiveTick`
  (params (DeltaSeconds :type "Float (single-precision)"))
  (bind _output_get (set `self.Time` (- (`self.Time`) DeltaSeconds)))
  (if (<= _output_get 0.0)
    (`self.Completed Game` :!label _label)
    (elif (<= (`self.Newspaper Ammo`) 0)
      (`KismetSystemLibrary.Delay` 5.0)
      (goto _label))))

(event `Completed Game`
  (set `self.Has Completed Game` true)
  (`GameplayStatics.SetGamePaused` true)
  (`WidgetLayoutLibrary.RemoveAllWidgets`)
  (bind _returnvalue (`|CreateWidget` "/Game/UI/WBP_Gameover.WBP_Gameover_C" (`GameplayStatics.GetPlayerController` 0)))
  (`UserWidget.AddToViewport` _returnvalue 0))

(fn `UserConstructionScript`)