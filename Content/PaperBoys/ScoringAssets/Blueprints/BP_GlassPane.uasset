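; BP_GlassPane is a breakable glass pane among the PaperBoys scoring assets that shatters the first time something overlaps its box.
; On that overlap it destroys the intact dummy pane and reveals a hidden fractured mesh, using a Broken flag to run only once.
; It then passes the overlapping actor to HandleChaos and plays the hit sound cue.
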(event `self.General Box.OnComponentBeginOverlap`
  (params (OverlappedComponent :type "PrimitiveComponent Object Reference") (OtherActor :type "Actor Object Reference") (OtherComp :type "PrimitiveComponent Object Reference") (OtherBodyIndex :type Integer) (bFromSweep :type Boolean) (SweepResult :type "HitResult Structure (by ref)"))
  (bind _hit_audio_component (`self.Hit Audio Component`))
  (if (not (`self.Broken`))
    (`ActorComponent.K2_DestroyComponent` (`self.Glass Pane Dummy`))
    (`SceneComponent.SetHiddenInGame` (`self.Fractured Mesh`) false false)
    (set `self.Broken` true)
    (`self.Handle Chaos` OtherActor)
    (`AudioComponent.SetSound` _hit_audio_component (`self.Hit Sound Cue`))
    (`AudioComponent.Play` _hit_audio_component 0.1)))

(fn `UserConstructionScript`
  (`parent.UserConstructionScript`))