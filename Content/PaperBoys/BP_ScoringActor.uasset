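; BP_ScoringActor is a vandalism target in the PaperBoys game, built to award points when a newspaper hits it.
; HandleChaos accepts only BP_Newspaper, then once enables physics on FracturedMesh, adds ScoreValue to GM_PaperBoy's score and sets HasVandalized.
; PlayAudio spawns an attached hit sound.
; The GeneralBox overlap event is empty here, with both calls left disconnected in the event graph.
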(event `self.General Box.OnComponentBeginOverlap`
  (params (OverlappedComponent :type "PrimitiveComponent Object Reference") (OtherActor :type "Actor Object Reference") (OtherComp :type "PrimitiveComponent Object Reference") (OtherBodyIndex :type Integer) (bFromSweep :type Boolean) (SweepResult :type "HitResult Structure (by ref)")))

(fn `Handle Chaos`
  (params (Actor :type "Actor Object Reference"))
  (bind _asgm_paper_boy (cast `/Game/PaperBoys/GM_PaperBoy` (`GameplayStatics.GetGameMode`) :!pure true))
  (cast `/Game/PaperBoys/BP_Newspaper` Actor)
  (if (`self.CanScore`)
    (`PrimitiveComponent.SetSimulatePhysics` (`self.Fractured Mesh`) true)
    (`/Game/PaperBoys/GM_PaperBoy.Add Score` _asgm_paper_boy (`self.Score Value`))
    (set `/Game/PaperBoys/GM_PaperBoy.Has Vandalized` true _asgm_paper_boy)
    (set `self.CanScore` false)))

(fn `Play Audio`
  (`GameplayStatics.SpawnSoundAttached` (`self.Hit Sound Cue`) (`self.Hit Audio Component`) "None" (`SceneComponent.K2_GetComponentLocation` (`self.Fractured Mesh`)) (struct) "KeepRelativeOffset" false 1.0 1.0 0.0 null null))

(fn `UserConstructionScript`)