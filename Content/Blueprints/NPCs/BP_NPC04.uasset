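; BP_NPC04 is an NPC Blueprint that reacts to being hit by a thrown newspaper.
; On overlap, it checks for actors tagged Newspaper moving at or above a minimum speed and passes them to HitByNewspaper, which is not defined in this graph.
; A PlaySound event assigns any valid sound to the Audio component and plays it from the start.
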(event `self.ReceiveActorBeginOverlap`
  (params (OtherActor :type "Actor Object Reference"))
  (if (`self.ActorHasTag` OtherActor "Newspaper")
    (if (>= (`KismetMathLibrary.VSize` (`self.GetVelocity` OtherActor)) 100.0)
      (`self.HitByNewspaper` OtherActor))))

(event `self.PlaySound`
  (params (SoundToPlay :type "SoundCue Object Reference"))
  (bind _audio (`self.Audio`))
  (`/Engine/EditorBlueprintResources/StandardMacros.IsValid` SoundToPlay
    (:`Is Valid`
      (`AudioComponent.SetSound` _audio SoundToPlay)
      (`AudioComponent.Play` _audio 0.0))))

(fn `UserConstructionScript`)