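; BP_Spawner periodically spawns cars on four routes and dogs around the player, using two looping timers started at BeginPlay.
; For each route it picks a random direction and spawns a random car class at the point farthest from the player.
; Each car gets the route reordered to start there, then begins driving.
; Dogs spawn at a random BP_CarSpawnPoint, filtered by minimum and maximum player distance.
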(event `self.ReceiveBeginPlay`
  (`self.SpawnCars`)
  (`KismetSystemLibrary.K2_SetTimer` null "SpawnCars" (`self.CarSpawnTimer`) true)
  (bind _outactors (`GameplayStatics.GetAllActorsOfClass` "/Game/Blueprints/Cars/BP_CarSpawnPoint.BP_CarSpawnPoint_C"))
  (set `self.SpawnPoints` _outactors)
  (`KismetSystemLibrary.K2_SetTimer` null "SpawnDog" (`self.DogSpawnTimer`) true))

(fn `GetFarthestSpawnPointFromPlayer`
  (params (Route :type "Array of Actor Object Reference"))
  (locals (FarthestActor :type "Actor Object Reference") (FarthestActorIndex :type Integer) (CarArray :type "Array of BaseCar Class Reference"))
  (bind _returnvalue (`GameplayStatics.GetPlayerPawn` 0))
  (bind _cararray (`local.CarArray`))
  (if (> (`KismetArrayLibrary.Array_Length` Route) 0)
    (for (_array_element _array_index) Route
      (if (== _array_index 0)
        (set `local.FarthestActor` _array_element)
        (set `local.FarthestActorIndex` 0)
        (elif (> (`self.GetDistanceTo` _array_element _returnvalue) (`self.GetDistanceTo` (`local.FarthestActor`) _returnvalue))
          (set `local.FarthestActor` _array_element)
          (set `local.FarthestActorIndex` _array_index))))
    (bind _returnvalue_2 (`|SpawnActorFromClass` (`|GetArrayItem` _cararray (`KismetMathLibrary.RandomInteger` (`KismetArrayLibrary.Array_Length` _cararray))) (`self.GetTransform` (`local.FarthestActor`)) "Undefined" "OverrideRootScale" null null))
    (`self.InitializeCar` _returnvalue_2 Route (`local.FarthestActorIndex`))
    (return)))

(fn `InitializeCar`
  (params (CarToInitialize :type "BaseCar Object Reference") (Route :type "Array of Actor Object Reference") (InitialIndex :type Integer))
  (locals (NewArray :type "Array of Actor Object Reference"))
  (for _index (range InitialIndex (+ (`KismetArrayLibrary.Array_LastIndex` Route) 1))
    (`KismetArrayLibrary.Array_Add` (`local.NewArray`) (`|GetArrayItem` Route _index)))
  (for _index_2 (range (+ InitialIndex 1))
    (`KismetArrayLibrary.Array_Add` (`local.NewArray`) (`|GetArrayItem` Route _index_2)))
  (`BaseCar.SetPathArray` CarToInitialize (`local.NewArray`))
  (`BaseCar.BeginDriving` CarToInitialize)
  (set `BaseCar.bSpawnedCar` true CarToInitialize))

(fn `RandomDirection`
  (returns (RightRoute :type Boolean))
  (switch `int` (`KismetMathLibrary.RandomInteger` 2)
    (:`0`
      (return true))
    (:`1`
      (return false))))

(fn `SpawnCarInRandomDirection`
  (params (RightDirection :type "Array of Actor Object Reference") (LeftDirection :type "Array of Actor Object Reference"))
  (bind _rightroute (`self.RandomDirection`))
  (if _rightroute
    (`self.GetFarthestSpawnPointFromPlayer` RightDirection)
    (else
      (`self.GetFarthestSpawnPointFromPlayer` LeftDirection))))

(fn `SpawnCars`
  (`self.SpawnCarInRandomDirection` (`self.Route01Right`) (`self.Route01Left`))
  (`self.SpawnCarInRandomDirection` (`self.Route02Right`) (`self.Route02Left`))
  (`self.SpawnCarInRandomDirection` (`self.Route03Right`) (`self.Route03Left`))
  (`self.SpawnCarInRandomDirection` (`self.Route04Right`) (`self.Route04Left`)))

(fn `SpawnDog`
  (locals (ObjectTypes :type "Array of EObjectTypeQuery Enum") (SpawnPoints_Copy :type "Array of /Game/Blueprints/Cars/BP_CarSpawnPoint Object Reference"))
  (bind _output_get (set `local.SpawnPoints_Copy` (`self.SpawnPoints`)))
  (for _array_element _output_get
    (bind _returnvalue (`self.GetDistanceTo` _array_element (`GameplayStatics.GetPlayerPawn` 0)))
    (if (or (< _returnvalue (`self.DogSpawnMinDistance`)) (> _returnvalue (`self.DogSpawnSphereRadius`)))
      (`KismetArrayLibrary.Array_RemoveItem` _output_get _array_element)))
  (bind _returnvalue_2 (`KismetArrayLibrary.Array_Length` _output_get))
  (`KismetSystemLibrary.PrintString` (`KismetStringLibrary.Conv_IntToString` _returnvalue_2))
  (if (> _returnvalue_2 0)
    (`|SpawnActorFromClass` "/Game/Blueprints/NPCs/BP_Dog.BP_Dog_C" (`self.GetTransform` (`KismetArrayLibrary.Array_Random` _output_get)) "Undefined" "OverrideRootScale" null null)))

(fn `UserConstructionScript`)