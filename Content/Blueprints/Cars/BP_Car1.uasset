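; BP_Car1 is a car that drives a looping spline route, begins stopping at stop signs and notifies any overlapping cart of a hit.
; CreateSplinePath spawns the spline from the path actor array, and Tick sweeps the car along it by moving speed while spinning the wheels from velocity.
; Chaos break events on six glass-pane child actors set the car Busted, with a timer later stopping its honk audio.
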(event `self.ReceiveActorBeginOverlap`
  (params (OtherActor :type "Actor Object Reference"))
  (cast `/Game/Blueprints/Cars/BP_StopSign` OtherActor
    (:`then`
      (`self.BeginStopping`))
    (:`CastFailed`
      (bind _asbp_cart (cast `/Game/PaperBoys/BP_Cart` OtherActor))
      (`PaperBoyInterface.PlayerHit` _asbp_cart self))))

(event `self.ReceiveBeginPlay`
  (`self.Bind to Chaos` (`self.Window 1_0`) (delegate `SetCarBusted`))
  (`self.Bind to Chaos` (`self.Window 6_0`) (delegate `SetCarBusted`))
  (`self.Bind to Chaos` (`self.Window 2_0`) (delegate `SetCarBusted`))
  (`self.Bind to Chaos` (`self.Window 5_0`) (delegate `SetCarBusted`))
  (`self.Bind to Chaos` (`self.Window 4_0`) (delegate `SetCarBusted`))
  (`self.Bind to Chaos` (`self.Window 3_0`) (delegate `SetCarBusted`)))

(event `SetCarBusted`
  (params (BreakEvent :type "ChaosBreakEvent Structure (by ref)"))
  (if (`|EnumInequality` (`self.GetCarState`) "Busted")
    (`self.SetCarState` "Busted")
    (`KismetSystemLibrary.K2_SetTimerDelegate` (delegate `StopBlaringHonk`) 15.0)))

(event `StopBlaringHonk`
  (`AudioComponent.Stop` (`self.Audio`)))

(event `self.ReceiveTick`
  (params (DeltaSeconds :type "Float (single-precision)"))
  (bind _spline (`/Game/Blueprints/Cars/BP_SplinePath.Spline` (`self.Spline Ref_0`)))
  (bind _returnvalue (`SplineComponent.GetSplineLength` (`/Game/Blueprints/Cars/BP_SplinePath.Spline` (`self.Spline Ref_0`))))
  (`self.RotateWheels` DeltaSeconds)
  (`/Engine/EditorBlueprintResources/StandardMacros.IsValid` (`self.Spline Ref_0`)
    (:`Is Valid`
      (bind _output_get (set `self.LerpAlpha_0` (+ (`self.LerpAlpha_0`) (/ (* DeltaSeconds (`self.GetMovingSpeed`)) _returnvalue))))
      (bind _returnvalue_2 (`KismetMathLibrary.Lerp` 0.0 _returnvalue _output_get))
      (`self.K2_SetActorTransform` (`KismetMathLibrary.MakeTransform` (`SplineComponent.GetLocationAtDistanceAlongSpline` _spline _returnvalue_2 "World") (`SplineComponent.GetRotationAtDistanceAlongSpline` _spline _returnvalue_2 "World")) true)
      (if (>= (`self.LerpAlpha_0`) 1.0)
        (set `self.LerpAlpha_0` 0.0)))))

(event `self.CreateSplinePath`
  (bind _returnvalue (`|SpawnActorFromClass` "/Game/Blueprints/Cars/BP_SplinePath.BP_SplinePath_C" (`self.GetTransform` (`|GetArrayItem` (`self.GetPathArray`))) "Undefined" "OverrideRootScale" null null))
  (set `self.Spline Ref_0` _returnvalue)
  (for _array_element (`self.GetPathArray`)
    (`SplineComponent.AddSplinePoint` (`/Game/Blueprints/Cars/BP_SplinePath.Spline` (`self.Spline Ref_0`)) (`self.K2_GetActorLocation` _array_element) "World" true)))

(event `self.PlaySound`
  (params (SoundToPlay :type "SoundCue Object Reference"))
  (bind _audio (`self.Audio`))
  (`/Engine/EditorBlueprintResources/StandardMacros.IsValid` SoundToPlay
    (:`Is Valid`
      (`AudioComponent.SetSound` _audio SoundToPlay)
      (`AudioComponent.Play` _audio 0.0))))

(fn `Bind to Chaos`
  (params (Window :type "ChildActorComponent Object Reference") (Delegate :type "Delegate (by ref)"))
  (bind _asbp_glass_pane (cast `/Game/PaperBoys/ScoringAssets/Blueprints/BP_GlassPane` (`ChildActorComponent.ChildActor` Window)))
  (add `GeometryCollectionComponent.OnChaosBreakEvent` (`/Game/PaperBoys/BP_ScoringActor.Fractured Mesh` _asbp_glass_pane) Delegate))

(fn `RotateWheels`
  (params (DeltaTime :type "Float (double-precision)"))
  (bind _returnvalue (* (* DeltaTime (`KismetMathLibrary.VSize` (* (`self.GetVelocity`) (`self.GetActorForwardVector`)))) -1.0))
  (`SceneComponent.K2_AddLocalRotation` (`self.WheelFR_0`) (`KismetMathLibrary.MakeRotator` 0.0 _returnvalue) false false)
  (`SceneComponent.K2_AddLocalRotation` (`self.WheelFL_0`) (`KismetMathLibrary.MakeRotator` 0.0 _returnvalue) false false)
  (`SceneComponent.K2_AddLocalRotation` (`self.WheelRR_0`) (`KismetMathLibrary.MakeRotator` 0.0 _returnvalue) false false)
  (`SceneComponent.K2_AddLocalRotation` (`self.WheelRL_0`) (`KismetMathLibrary.MakeRotator` 0.0 _returnvalue) false false))

(fn `UserConstructionScript`)