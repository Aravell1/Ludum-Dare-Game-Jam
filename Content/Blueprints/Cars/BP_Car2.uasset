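; Car actor that drives a looping route along a spline and reacts to stop signs.
; CreateSplinePath spawns a BP_SplinePath at the first path actor and adds a spline point at each path actor's location.
; Tick advances a length-normalized alpha by moving speed, sweeps the car along the spline, and spins four wheels from forward-scaled velocity.
; Overlapping a BP_StopSign calls BeginStopping, which is defined outside this graph.
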(event `self.ReceiveActorBeginOverlap`
  (params (OtherActor :type "Actor Object Reference"))
  (cast `/Game/Blueprints/Cars/BP_StopSign` OtherActor)
  (`self.BeginStopping`))

(event `self.ReceiveTick`
  (params (DeltaSeconds :type "Float (single-precision)"))
  (bind _spline (`/Game/Blueprints/Cars/BP_SplinePath.Spline` (`self.Spline Ref`)))
  (bind _returnvalue (`SplineComponent.GetSplineLength` (`/Game/Blueprints/Cars/BP_SplinePath.Spline` (`self.Spline Ref`))))
  (`self.RotateWheels` DeltaSeconds)
  (`/Engine/EditorBlueprintResources/StandardMacros.IsValid` (`self.Spline Ref`)
    (:`Is Valid`
      (bind _output_get (set `self.LerpAlpha` (+ (`self.LerpAlpha`) (/ (* DeltaSeconds (`self.GetMovingSpeed`)) _returnvalue))))
      (bind _returnvalue_2 (`KismetMathLibrary.Lerp` 0.0 _returnvalue _output_get))
      (`self.K2_SetActorTransform` (`KismetMathLibrary.MakeTransform` (`SplineComponent.GetLocationAtDistanceAlongSpline` _spline _returnvalue_2 "World") (`SplineComponent.GetRotationAtDistanceAlongSpline` _spline _returnvalue_2 "World")) true)
      (if (>= (`self.LerpAlpha`) 1.0)
        (set `self.LerpAlpha` 0.0)))))

(event `self.CreateSplinePath`
  (bind _returnvalue (`|SpawnActorFromClass` "/Game/Blueprints/Cars/BP_SplinePath.BP_SplinePath_C" (`self.GetTransform` (`|GetArrayItem` (`self.GetPathArray`))) "Undefined" "OverrideRootScale" null null))
  (set `self.Spline Ref` _returnvalue)
  (for _array_element (`self.GetPathArray`)
    (`SplineComponent.AddSplinePoint` (`/Game/Blueprints/Cars/BP_SplinePath.Spline` (`self.Spline Ref`)) (`self.K2_GetActorLocation` _array_element) "World" true)))

(fn `RotateWheels`
  (params (DeltaTime :type "Float (double-precision)"))
  (bind _returnvalue (* (* DeltaTime (`KismetMathLibrary.VSize` (* (`self.GetVelocity`) (`self.GetActorForwardVector`)))) -1.0))
  (`SceneComponent.K2_AddLocalRotation` (`self.WheelFR`) (`KismetMathLibrary.MakeRotator` 0.0 _returnvalue) false false)
  (`SceneComponent.K2_AddLocalRotation` (`self.WheelFL`) (`KismetMathLibrary.MakeRotator` 0.0 _returnvalue) false false)
  (`SceneComponent.K2_AddLocalRotation` (`self.WheelRR`) (`KismetMathLibrary.MakeRotator` 0.0 _returnvalue) false false)
  (`SceneComponent.K2_AddLocalRotation` (`self.WheelRL`) (`KismetMathLibrary.MakeRotator` 0.0 _returnvalue) false false))

(fn `UserConstructionScript`)